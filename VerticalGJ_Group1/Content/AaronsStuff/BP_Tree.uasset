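; BP_Tree is a tree actor that tracks health and shows it on its TreeHealth text.
; The construction script displays the starting Health.
; Each time a BP_ThirdPersonCharacter begins overlapping its Box, UpdateDamageHealth subtracts a fixed amount and refreshes the text.
; The zero check runs before subtraction, so Health can dip negative until the next hit resets it, and depletion triggers nothing else.
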(event `self.Box.OnComponentBeginOverlap`
  (params (OverlappedComponent :type "PrimitiveComponent Object Reference") (OtherActor :type "Actor Object Reference") (OtherComp :type "PrimitiveComponent Object Reference") (OtherBodyIndex :type Integer) (bFromSweep :type Boolean) (SweepResult :type "HitResult Structure (by ref)"))
  (cast `/Game/ThirdPerson/Blueprints/BP_ThirdPersonCharacter` OtherActor)
  (`self.UpdateDamageHealth` 20.0))

(fn `UpdateDamageHealth`
  (params (EnemyDamageAmount :type "Float (double-precision)"))
  (bind _health (`self.Health`))
  (if (<= _health 0.0)
    (bind _output_get (set `self.Health` 0.0))
    (`self.UpdateHealthText` _output_get)
    (else
      (bind _output_get_2 (set `self.Health` (- _health EnemyDamageAmount)))
      (`self.UpdateHealthText` _output_get_2))))

(fn `UpdateHealthText`
  (params (Value :type "Float (double-precision)"))
  (`TextRenderComponent.K2_SetText` (`self.TreeHealth`) (`KismetTextLibrary.Conv_DoubleToText` Value "HalfToEven")))

(fn `UserConstructionScript`
  (`TextRenderComponent.K2_SetText` (`self.TreeHealth`) (`KismetTextLibrary.Conv_DoubleToText` (`self.Health`) "HalfToEven")))