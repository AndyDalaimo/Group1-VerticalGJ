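; BP_Tree2 is a tree with health that ends the game when it runs out.
; While an actor tagged "Tree" overlaps its Box, a looping timer drains health each second and updates the player's HUD, showing game over through the GameInstance at zero.
; UpdateDamageHealth offers separate damage without HUD or game-over handling.
; UpdateHealingHealth is empty, HasCollision always returns false, and the cached enemy reference is unused.
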(event `self.ReceiveBeginPlay`
  ;[0 0 0] Set Refs
  (bind _returnvalue (`GameplayStatics.GetActorOfClass` "/Script/VerticalGJ_Group1.AIEnemyCharacter"))
  (set `self.EnemyRef` _returnvalue)
  (bind _returnvalue_2 (`GameplayStatics.GetActorOfClass` "/Game/ThirdPerson/Blueprints/BP_Player.BP_Player_C"))
  (set `self.PlayerRef` _returnvalue_2)
  (bind _asmy_game_instance (cast `MyGameInstance` (`GameplayStatics.GetGameInstance`)))
  (set `self.GameInstanceRef` _asmy_game_instance))

(event `self.Box.OnComponentBeginOverlap`
  (params (OverlappedComponent :type "PrimitiveComponent Object Reference") (OtherActor :type "Actor Object Reference") (OtherComp :type "PrimitiveComponent Object Reference") (OtherBodyIndex :type Integer) (bFromSweep :type Boolean) (SweepResult :type "HitResult Structure (by ref)"))
  ;[0 0 0] Attack & Destroy Tree
  (if (`self.ActorHasTag` OtherActor "Tree")
    (bind _returnvalue (`KismetSystemLibrary.K2_SetTimerDelegate` (delegate `DamageTree`) 1.0 true))))

(event `DamageTree`
  ;[0 0 0] Attack & Destroy Tree
  (bind _output_get (set `self.Health` (- (`self.Health`) 15.0)))
  (`/Game/UI/WBP_HUD.UpdateHealthUI` (`/Game/ThirdPerson/Blueprints/BP_Player.HUDRef` (`self.PlayerRef`)) _output_get (`self.MaxHealth`))
  (if (<= _output_get 0.0)
    (`KismetSystemLibrary.K2_ClearAndInvalidateTimerHandle` (stale `self.Box.OnComponentBeginOverlap` _returnvalue))
    (`MyGameInstance.ShowGameOverWidget` (`self.GameInstanceRef`))))

(event `self.Box.OnComponentEndOverlap`
  (params (OverlappedComponent :type "PrimitiveComponent Object Reference") (OtherActor :type "Actor Object Reference") (OtherComp :type "PrimitiveComponent Object Reference") (OtherBodyIndex :type Integer))
  (if (`self.ActorHasTag` OtherActor "Tree")
    (`KismetSystemLibrary.K2_ClearAndInvalidateTimerHandle` (stale `self.Box.OnComponentBeginOverlap` _returnvalue))))

(fn `HasCollision`
  (returns (HasCollision :type Boolean))
  (return false))

(fn `UpdateDamageHealth`
  (params (EnemyDamageAmount :type "Float (double-precision)"))
  (bind _health (`self.Health`))
  (if (<= _health 0.0)
    (set `self.Health` 0.0)
    (else
      (set `self.Health` (- _health EnemyDamageAmount)))))

(fn `UpdateHealingHealth`)

(fn `UserConstructionScript`)