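; BP_TestNPC is a test NPC Blueprint that appears to be an unfinished prototype for healing near a referenced tree.
; When its sphere begins overlapping that tree, it starts a one-second, non-looping timer bound to a heal event.
; The heal event is empty, and disconnected leftover nodes for changing Health and updating the player's health UI never run.
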(event `self.Sphere1.OnComponentBeginOverlap`
  (params (OverlappedComponent :type "PrimitiveComponent Object Reference") (OtherActor :type "Actor Object Reference") (OtherComp :type "PrimitiveComponent Object Reference") (OtherBodyIndex :type Integer) (bFromSweep :type Boolean) (SweepResult :type "HitResult Structure (by ref)"))
  (if (== OtherActor (`self.TreeRef`))
    (`KismetSystemLibrary.K2_SetTimerDelegate` (delegate `HealEvent`) 1.0)))

(event `HealEvent`)

(fn `UserConstructionScript`)