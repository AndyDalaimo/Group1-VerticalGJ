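; BP_Tree2 is a destructible tree that loses health over time once the player touches it.
; Player overlap with its Box starts a looping one-second timer, with no end-overlap handler to stop it.
; Each tick subtracts health, pushes the tree's values to the player's WBMain health UI, and destroys the tree at zero.
; DestroyTreeforReal destroys it immediately; AnyDamage is empty and the cached AIEnemy reference is unused.
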(event `self.ReceiveBeginPlay`
  (bind _returnvalue (`GameplayStatics.GetActorOfClass` "/Script/VerticalGJ_Group1.AIEnemy"))
  (set `self.EnemyRef` _returnvalue)
  (bind _returnvalue_2 (`GameplayStatics.GetActorOfClass` "/Game/AaronsStuff/TestCharacter/BP_TestCharacter.BP_TestCharacter_C"))
  (set `self.PlayerRef` _returnvalue_2))

(event `/Game/AaronsStuff/TestCharacter/BPI_Tree2Interface.DestroyTreeForReal`
  (`self.K2_DestroyActor`))

(event `self.Box.OnComponentBeginOverlap`
  (params (OverlappedComponent :type "PrimitiveComponent Object Reference") (OtherActor :type "Actor Object Reference") (OtherComp :type "PrimitiveComponent Object Reference") (OtherBodyIndex :type Integer) (bFromSweep :type Boolean) (SweepResult :type "HitResult Structure (by ref)"))
  (if (== OtherActor (`self.PlayerRef`))
    (bind _returnvalue (`KismetSystemLibrary.K2_SetTimerDelegate` (delegate `DamageTree`) 1.0 true))))

(event `DamageTree`
  (bind _output_get (set `self.Health` (- (`self.Health`) 100.0)))
  (`/Game/UI/WBP_HUD.UpdateHealthUI` (`/Game/AaronsStuff/TestCharacter/BP_TestCharacter.WB_Main` (`self.PlayerRef`)) _output_get (`self.MaxHealth`))
  (if (<= _output_get 0.0)
    (`KismetSystemLibrary.K2_ClearAndInvalidateTimerHandle` (stale `self.Box.OnComponentBeginOverlap` _returnvalue))
    (`self.K2_DestroyActor`)))

(event `self.ReceiveAnyDamage`
  (params (Damage :type "Float (single-precision)") (DamageType :type "DamageType Object Reference") (InstigatedBy :type "Controller Object Reference") (DamageCauser :type "Actor Object Reference")))

(fn `UserConstructionScript`)