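; BP_AIEnemy is an enemy actor that tracks its health and is destroyed when the player depletes it.
; On BeginPlay it copies type, health and damage from its EnemyProperties struct.
; AnyDamage only counts hits whose damage causer is the player character itself, clamps health between zero and the maximum, and destroys the actor at zero.
; No AI behavior or attack logic is implemented in these graphs.
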(event `self.ReceiveAnyDamage`
  (params (Damage :type "Float (single-precision)") (DamageType :type "DamageType Object Reference") (InstigatedBy :type "Controller Object Reference") (DamageCauser :type "Actor Object Reference"))
  ;[1 1 1] Dmg + Death
  (if (== DamageCauser (`GameplayStatics.GetPlayerCharacter` 0))
    (bind _output_get (set `self.Current Health` (`KismetMathLibrary.FClamp` (- (`self.Current Health`) Damage) 0.0 (`self.Max Health`))))
    (if (== _output_get 0.0)
      (`self.K2_DestroyActor`))))

(event `self.ReceiveBeginPlay`
  (bind (_type _hp _damage) (break `AIEnemyProperties` (`self.EnemyProperties`)))
  (bind _returnvalue (`KismetMathLibrary.Conv_IntToDouble` _hp))
  (set `self.Type` _type)
  (set `self.Max Health` _returnvalue)
  (set `self.Current Health` (`KismetMathLibrary.FClamp` _returnvalue 0.0 (`self.Max Health`)))
  (set `self.Damage` _damage))

(fn `UserConstructionScript`)