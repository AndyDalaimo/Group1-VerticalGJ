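; BP_SmallTree_4 is a purchasable tree plot that moves itself to the fifth entry (index 4) of SpawnLocations on BeginPlay and shows its berry cost.
; When the player overlaps its box with enough PlayerResources, it flags the purchase, reveals the tree mesh, calls TreePlanted and hides the cost text.
; A Purchased flag blocks repeat buys, and UpdateText refreshes the cost label.
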(event `self.ReceiveBeginPlay`
  (`parent.ReceiveBeginPlay`)
  (bind _output_get (set `self.ThisTreeSpawnLocation` (`|GetArrayItem` (`self.SpawnLocations`) 4)))
  (`self.K2_SetActorLocation` _output_get)
  (`TextRenderComponent.K2_SetText` (`self.CostText`) (`|FormatText` "Plant Tree: {COST} Berries " (`self.CostOfTree`))))

(event `self.Box.OnComponentBeginOverlap`
  (params (OverlappedComponent :type "PrimitiveComponent Object Reference") (OtherActor :type "Actor Object Reference") (OtherComp :type "PrimitiveComponent Object Reference") (OtherBodyIndex :type Integer) (bFromSweep :type Boolean) (SweepResult :type "HitResult Structure (by ref)"))
  (bind _playerref (`self.PlayerRef`))
  (if (and (== OtherActor _playerref) (>= (`MyGameInstance.PlayerResources` (`self.GameInstanceRef`)) (`self.CostOfTree`)) (not (`self.Purchased`)))
    (set `/Game/ThirdPerson/Blueprints/BP_Player.Purchase` true _playerref)
    (`SceneComponent.SetVisibility` (`self.StaticMesh`) true false)
    (set `self.Purchased` true)
    (`KismetSystemLibrary.PrintString` "Bought this tree")
    (`self.TreePlanted`)
    (`SceneComponent.SetVisibility` (`self.CostText`) false false)))

(fn `UpdateText`
  (`TextRenderComponent.K2_SetText` (`self.CostText`) (`|FormatText` "Plant Tree: {COST} Berries " (`self.CostOfTree`))))

(fn `UserConstructionScript`
  (`parent.UserConstructionScript`))