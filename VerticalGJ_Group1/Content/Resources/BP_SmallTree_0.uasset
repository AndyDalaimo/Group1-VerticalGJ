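; Small plantable tree, a child Blueprint that moves to the first spawn location on BeginPlay and shows its berry cost as text.
; When the player overlaps its box with enough resources, it reveals the tree and bush meshes, marks itself purchased and calls TreePlanted.
; Once purchased, its enemy hurt box only prints a debug message for overlapping actors tagged "Tree".
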(event `self.ReceiveBeginPlay`
  (`parent.ReceiveBeginPlay`)
  (bind _output_get (set `self.ThisTreeSpawnLocation` (`|GetArrayItem` (`self.SpawnLocations`))))
  (`self.K2_SetActorLocation` _output_get)
  (`TextRenderComponent.K2_SetText` (`self.CostText`) (`|FormatText` "Plant Tree: {COST} Berries " (`self.CostOfTree`))))

(event `self.Box.OnComponentBeginOverlap`
  (params (OverlappedComponent :type "PrimitiveComponent Object Reference") (OtherActor :type "Actor Object Reference") (OtherComp :type "PrimitiveComponent Object Reference") (OtherBodyIndex :type Integer) (bFromSweep :type Boolean) (SweepResult :type "HitResult Structure (by ref)"))
  (if (and (== OtherActor (`self.PlayerRef`)) (>= (`MyGameInstance.PlayerResources` (`self.GameInstanceRef`)) (`self.CostOfTree`)) (not (`self.Purchased`)))
    (`self.SetVisibilityOfMeshes`)
    (set `self.Purchased` true)
    (`KismetSystemLibrary.PrintString` "Bought this tree")
    (`self.TreePlanted`)))

(event `self.EnemyHurtBox.OnComponentBeginOverlap`
  (params (OverlappedComponent :type "PrimitiveComponent Object Reference") (OtherActor :type "Actor Object Reference") (OtherComp :type "PrimitiveComponent Object Reference") (OtherBodyIndex :type Integer) (bFromSweep :type Boolean) (SweepResult :type "HitResult Structure (by ref)"))
  (if (and (`self.Purchased`) (`self.ActorHasTag` OtherActor "Tree"))
    (`KismetSystemLibrary.PrintString` "Enemy Hurt")))

(fn `SetVisibilityOfMeshes`
  (`SceneComponent.SetVisibility` (`self.StaticMesh`) true false)
  (`SceneComponent.SetVisibility` (`self.Bush`) true false)
  (`SceneComponent.SetVisibility` (`self.Bush1`) true false)
  (`SceneComponent.SetVisibility` (`self.Bush2`) true false))

(fn `UpdateText`
  (`TextRenderComponent.K2_SetText` (`self.CostText`) (`|FormatText` "Plant Tree: {COST} Berries " (`self.CostOfTree`))))

(fn `UserConstructionScript`
  (`parent.UserConstructionScript`))