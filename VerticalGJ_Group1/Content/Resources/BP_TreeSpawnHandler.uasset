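; BP_TreeSpawnHandler charges the player's resources when a tree is planted and raises the price of the next one.
; On BeginPlay it caches the MyGameInstance and the BP_Player actor.
; TreePlanted subtracts the current cost through the game instance, then adds a fixed increment to that cost.
; The file contains no spawning logic and does not use the cached player reference.
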(event `self.ReceiveBeginPlay`
  (bind _asmy_game_instance (cast `MyGameInstance` (`GameplayStatics.GetGameInstance`)))
  (set `self.GameInstanceRef` _asmy_game_instance)
  (bind _returnvalue (`GameplayStatics.GetActorOfClass` "/Game/ThirdPerson/Blueprints/BP_Player.BP_Player_C"))
  (set `self.PlayerRef` _returnvalue))

(fn `TreePlanted`
  (`MyGameInstance.SubtractResources` (`self.GameInstanceRef`) (`self.CostOfTree`))
  (set `self.CostOfTree` (+ (`self.CostOfTree`) (`self.CostIncrease`))))

(fn `UserConstructionScript`)